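; First-play subsystem that runs the new-player guide state machine and persists its progress in the save game.
; LoadState creates BP_GuideStateMachine_FirstPlay with the game instance as context, restores saved active states and starts it, unless already finished or created.
; SaveState writes all active state GUIDs to the save instance and saves the game.
; IsFinished checks the saved game-state tags for GameState.FirstPlayFinished.
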(fn LoadState
  (if (not (CallFunction|IsFinished))
    (Utilities|IsValid (Variables|Default|GetStateMachineInstance)
      (:Is%20Not%20Valid
        (bind _returnvalue (Class|SMBlueprintUtils|CreateStateMachineInstance "/Game/Blueprints/FirstPlayGuide/BP_GuideStateMachine_FirstPlay.BP_GuideStateMachine_FirstPlay_C" (Game|GetGameInstance) true))
        (Variables|Default|SetStateMachineInstance _returnvalue)
        (Class|SMInstance|LoadfromMultipleStates (Variables|Default|GetStateMachineInstance) (Variables|/Game/Blueprints/Framework/SaveGame/SaveGameTemplate.SaveGameTemplate_C|GetFirstPlayStates (Variables|/Game/Blueprints/Framework/BP_GameInstance.BP_GameInstance_C|GetSaveGameInstance (.AsBP%20Game%20Instance (Utilities|Casting|CastToBP_GameInstance (Game|GetGameInstance))))) true)
        (Class|SMInstance|Start (Variables|Default|GetStateMachineInstance))))))

(fn SaveState
  (bind _returnvalue (Game|GetGameInstance))
  (bind _asbp_game_instance (Utilities|Casting|CastToBP_GameInstance _returnvalue))
  (Variables|/Game/Blueprints/Framework/SaveGame/SaveGameTemplate.SaveGameTemplate_C|SetFirstPlayStates (Variables|/Game/Blueprints/Framework/BP_GameInstance.BP_GameInstance_C|GetSaveGameInstance _asbp_game_instance) (Class|SMInstance|GetAllActiveStateGuids (Variables|Default|GetStateMachineInstance)))
  (Default|SaveGame _asbp_game_instance))

(fn IsFinished
  (return (GameplayTags|HasTag (Variables|/Game/Blueprints/Framework/SaveGame/SaveGameTemplate.SaveGameTemplate_C|GetGameSTateTags (Variables|/Game/Blueprints/Framework/BP_GameInstance.BP_GameInstance_C|GetSaveGameInstance (.AsBP%20Game%20Instance (Utilities|Casting|CastToBP_GameInstance (Game|GetGameInstance))))) "(TagName=\"GameState.FirstPlayFinished\")" true)))