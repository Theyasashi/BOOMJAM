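; LoadManager is a level bootstrap actor that loads the saved game and spawns one player character and one enemy for the hex-tile map.
; It registers both in BP_GameStateInGame, then places and joins them to the first and last grass tiles, waiting for HexManager's create-finish event if none exist yet.
; It also listens for Test and Health attribute-change broadcasts, printing debug strings on specific value transitions, gated by DoOnce nodes.
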(event Custom|自定义事件_0
  (bind _as_bp_game_state_in_game (Variables|Default|GetAs%20BP%20Game%20State%20In%20Game))
  (bind _enemycharactor (Variables|/Game/Blueprints/Framework/BP_GameStateInGame.BP_GameStateInGame_C|GetEnemyCharactor _as_bp_game_state_in_game))
  (bind _playercontrolcharactor (Variables|/Game/Blueprints/Framework/BP_GameStateInGame.BP_GameStateInGame_C|GetPlayerControlCharactor _as_bp_game_state_in_game))
  (bind _output (Utilities|Array|Get(acopy) _playercontrolcharactor))
  (bind _output_2 (Utilities|Array|Get(acopy) _enemycharactor))
  (bind _outactors (Actor|GetAllActorsOfClass "/Game/SqrSLG/Blueprints/Bp_HexTile_Grass.Bp_HexTile_Grass_C"))
  (bind _output_get (Variables|Default|SetOut%20Actors _outactors))
  (Transformation|SetActorLocation _output (Transformation|GetActorLocation (Utilities|Array|Get(acopy) _output_get)) false false)
  (Default|Join (Utilities|Array|Get(acopy) _output_get) _output)
  (Transformation|SetActorLocation _output_2 (Transformation|GetActorLocation (Utilities|Array|Get(acopy) _output_get (- (Utilities|Array|Length _output_get) 1))) false false)
  (Default|Join (Utilities|Array|Get(acopy) _output_get (- (Utilities|Array|Length _output_get) 1)) _output_2))

(event EventBeginPlay
  (bind _returnvalue (Game|GetGameInstance))
  (bind _returnvalue_2 (Guid|NewGuid))
  (bind _self self)
  (bind _asbp_game_instance (Utilities|Casting|CastToBP_GameInstance _returnvalue))
  (bind _globalbroadcastsubsystem (Variables|/Game/Blueprints/Framework/BP_GameInstance.BP_GameInstance_C|GetGlobalBroadCastSubSystem _asbp_game_instance))
  (|CallParentFunction)
  (Utilities|FlowControl|Sequence
    (:then_0
      (bind _asbp_game_state_in_game (Utilities|Casting|CastToBP_GameStateInGame (Game|GetGameState)))
      (Variables|Default|SetAs%20BP%20Game%20State%20In%20Game _asbp_game_state_in_game))
    (:then_1
      (Default|LoadGame _asbp_game_instance)
      (Default|监听Listen _globalbroadcastsubsystem "(TagName=\"Attribute.Test.Event.Change\")" _self)
      (Default|监听Listen _globalbroadcastsubsystem "(TagName=\"Attribute.Health.Event.Change\")" _self)
      (bind _returnvalue_3 (Game|SpawnActorfromClass "/Game/Blueprints/Charactor/bp_Charactor1.bp_Charactor1_C" (Math|Transform|MakeTransform "0, 0, 0" "0, 0, 0" "1,1,1") "Undefined" 0 _returnvalue_2 0))
      (Utilities|Array|Add (Variables|/Game/Blueprints/Framework/BP_GameStateInGame.BP_GameStateInGame_C|GetPlayerControlCharactor (Variables|Default|GetAs%20BP%20Game%20State%20In%20Game)) _returnvalue_3)
      (bind _returnvalue_4 (Game|SpawnActorfromClass "/Game/Blueprints/Charactor/bp_Enemy1.bp_Enemy1_C" (Math|Transform|MakeTransform "0, 0, 0" "0, 0, 0" "1,1,1") "Undefined" 0 _returnvalue_2 0))
      (Utilities|Array|Add (Variables|/Game/Blueprints/Framework/BP_GameStateInGame.BP_GameStateInGame_C|GetEnemyCharactor (Variables|Default|GetAs%20BP%20Game%20State%20In%20Game)) _returnvalue_4))
    (:then_2
      (bind _outactors (Actor|GetAllActorsOfClass "/Game/SqrSLG/Blueprints/Bp_HexTile_Grass.Bp_HexTile_Grass_C"))
      (if (Utilities|Array|IsValidIndex _outactors)
        (bind _outactors_2 (Actor|GetAllActorsOfClass "/Game/SqrSLG/Blueprints/Bp_HexTile_Grass.Bp_HexTile_Grass_C"))
        (bind _output_get (Variables|Default|SetOut%20Actors _outactors_2))
        (Transformation|SetActorLocation (Utilities|Array|Get(acopy) (Variables|/Game/Blueprints/Framework/BP_GameStateInGame.BP_GameStateInGame_C|GetPlayerControlCharactor (Variables|Default|GetAs%20BP%20Game%20State%20In%20Game))) (Transformation|GetActorLocation (Utilities|Array|Get(acopy) _output_get)) false false)
        (Default|Join (Utilities|Array|Get(acopy) _output_get) (Utilities|Array|Get(acopy) (Variables|/Game/Blueprints/Framework/BP_GameStateInGame.BP_GameStateInGame_C|GetPlayerControlCharactor (Variables|Default|GetAs%20BP%20Game%20State%20In%20Game))))
        (Transformation|SetActorLocation (Utilities|Array|Get(acopy) (Variables|/Game/Blueprints/Framework/BP_GameStateInGame.BP_GameStateInGame_C|GetEnemyCharactor (Variables|Default|GetAs%20BP%20Game%20State%20In%20Game))) (Transformation|GetActorLocation (Utilities|Array|Get(acopy) _output_get (- (Utilities|Array|Length _output_get) 1))) false false)
        (Default|Join (Utilities|Array|Get(acopy) _output_get (- (Utilities|Array|Length _output_get) 1)) (Utilities|Array|Get(acopy) (Variables|/Game/Blueprints/Framework/BP_GameStateInGame.BP_GameStateInGame_C|GetEnemyCharactor (Variables|Default|GetAs%20BP%20Game%20State%20In%20Game))))
        (else
          (EventDispatchers|BindEventtoCreateFinish (Variables|Default|GetHexManager) (delegate Custom|自定义事件_0)))))))

(event EventTick
  (params (DeltaSeconds :type Float%20%28single-precision%29)))

(event EventBroadcast
  (params (EventTag :type Gameplay%20Tag%20Structure) (标签参数 :type Gameplay%20Tag%20Container%20Structure) (对象参数 :type Broadcast%20Parameter%20Base%20Object%20Reference))
  (if (== EventTag "(TagName=\"Attribute.Test.Event.Change\")")
    (Utilities|FlowControl|Sequence
      (:then_0
        (Utilities|FlowControl|DoOnce true :!label _label
          (:Completed
            (bind _asbp_on_attribute_value_change_parameter_float (Utilities|Casting|CastToBP_OnAttributeValueChangeParameter_Float 对象参数))
            (if (and (== (Variables|/Game/Blueprints/Core/Attribute/BP_OnAttributeValueChangeParameter_Float.BP_OnAttributeValueChangeParameter_Float_C|GetOldValue _asbp_on_attribute_value_change_parameter_float) 11.0) (== (Variables|/Game/Blueprints/Core/Attribute/BP_OnAttributeValueChangeParameter_Float.BP_OnAttributeValueChangeParameter_Float_C|GetNewValue _asbp_on_attribute_value_change_parameter_float) 1e+01))
              (Development|PrintString "OK2")))))
      (:then_1
        (Utilities|FlowControl|DoOnce false
          (:Completed
            (bind _asbp_on_attribute_value_change_parameter_float_2 (Utilities|Casting|CastToBP_OnAttributeValueChangeParameter_Float 对象参数))
            (if (and (== (Variables|/Game/Blueprints/Core/Attribute/BP_OnAttributeValueChangeParameter_Float.BP_OnAttributeValueChangeParameter_Float_C|GetOldValue _asbp_on_attribute_value_change_parameter_float_2) 1e+01) (== (Variables|/Game/Blueprints/Core/Attribute/BP_OnAttributeValueChangeParameter_Float.BP_OnAttributeValueChangeParameter_Float_C|GetNewValue _asbp_on_attribute_value_change_parameter_float_2) 11.0))
              (Development|PrintString "OK1")
              (goto _label Reset))))))
    (elif (== EventTag "(TagName=\"Attribute.Health.Event.Change\")")
      (Utilities|FlowControl|Sequence
        (:then_0
          (Utilities|FlowControl|DoOnce true :!label _label_2
            (:Completed
              (bind _asbp_on_attribute_value_change_parameter_float_3 (Utilities|Casting|CastToBP_OnAttributeValueChangeParameter_Float 对象参数))
              (if (and (== (Variables|/Game/Blueprints/Core/Attribute/BP_OnAttributeValueChangeParameter_Float.BP_OnAttributeValueChangeParameter_Float_C|GetOldValue _asbp_on_attribute_value_change_parameter_float_3) 11.0) (== (Variables|/Game/Blueprints/Core/Attribute/BP_OnAttributeValueChangeParameter_Float.BP_OnAttributeValueChangeParameter_Float_C|GetNewValue _asbp_on_attribute_value_change_parameter_float_3) 1e+01))
                (Development|PrintString "OK5")))))
        (:then_1
          (bind _asbp_on_attribute_value_change_parameter_float_4 (Utilities|Casting|CastToBP_OnAttributeValueChangeParameter_Float 对象参数))
          (if (and (== (Variables|/Game/Blueprints/Core/Attribute/BP_OnAttributeValueChangeParameter_Float.BP_OnAttributeValueChangeParameter_Float_C|GetOldValue _asbp_on_attribute_value_change_parameter_float_4) 1e+01) (== (Variables|/Game/Blueprints/Core/Attribute/BP_OnAttributeValueChangeParameter_Float.BP_OnAttributeValueChangeParameter_Float_C|GetNewValue _asbp_on_attribute_value_change_parameter_float_4) 11.0))
            (Development|PrintString "OK4")
            (goto _label_2 Reset)))))))

(event Collision|EventActorBeginOverlap
  (params (OtherActor :type Actor%20Object%20Reference))
  (|CallParentFunction OtherActor) ; 此节点被禁用，将不会被调用。\n从引脚连出引线来编译功能。
)

(fn ConstructionScript
  (|CallParentFunction))