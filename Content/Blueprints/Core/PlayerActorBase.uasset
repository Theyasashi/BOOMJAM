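; Base player actor for a hex-tile game, handling saved position and the actions available on a target tile.
; On BeginPlay it reads the position attribute from AttributeComponent if its Id is valid, otherwise generates an Id and saves the position.
; GetActions skips the occupied tile and tiles near world origin, then returns gameplay tags: Move, plus Attack against bp_Enemy1 occupants, each requiring the matching AbilityComponent tag.
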(event EventBeginPlay
  (bind _attribute (Default|Get属性对象 (Variables|Default|GetAttributeComponent) "(TagName=\"Attribute.Position\")"))
  (bind _asattribute_position (Utilities|Casting|CastToAttribute_Position _attribute))
  (if (Guid|IsValidGuid (Variables|Default|GetId))
    (Default|GetValue _asattribute_position) ; 获得存档位置
    (else
      (Variables|Default|SetId (Guid|NewGuid))
      (Default|Save _asattribute_position) ; 保存位置到存档
    )))

(event Collision|EventActorBeginOverlap
  (params (OtherActor :type Actor%20Object%20Reference)))

(event EventTick
  (params (DeltaSeconds :type Float%20%28single-precision%29)))

(fn ConstructionScript
  (|CallParentFunction))

(fn GetActions
  (params (TargetHexTile :type Bp%20Hex%20Tile%20Grass%20Object%20Reference))
  (bind _returnvalue (GameplayTags|MakeLiteralGameplayTag "(TagName=\"Ability.Attack\")"))
  (bind _returnvalue_2 (GameplayTags|MakeLiteralGameplayTag "(TagName=\"Ability.Move\")"))
  (bind _abilitycomponent (Variables|Default|GetAbilityComponent))
  (bind _tags (Variables|/Game/Blueprints/Core/Components/AbilityComponent.AbilityComponent_C|GetTags _abilitycomponent))
  (Utilities|FlowControl|Sequence
    (:then_0
      (if (not (== TargetHexTile (Variables|Default|GetStandHexTitle)))
        (if (> (Math|Vector|Distance2D(Vector) (Transformation|GetActorLocation TargetHexTile) "0, 0, 0") 1e+02)
          (Utilities|FlowControl|Sequence
            (:then_0
              (if (GameplayTags|HasTag _tags _returnvalue_2 true)
                (GameplayTags|AddGameplayTag (LocalVariables|GetL_Result) _returnvalue_2 :!class /Script/GameplayTags.BlueprintGameplayTagLibrary)))
            (:then_1
              (Utilities|Casting|CastTobp_Enemy1 (Variables|/Game/SqrSLG/Blueprints/Bp_HexTile_Grass.Bp_HexTile_Grass_C|GetActorOnHexTile TargetHexTile))
              (if (GameplayTags|HasTag _tags _returnvalue true)
                (GameplayTags|AddGameplayTag (LocalVariables|GetL_Result) _returnvalue :!class /Script/GameplayTags.BlueprintGameplayTagLibrary)))))))
    (:then_1
      (return (LocalVariables|GetL_Result)))))