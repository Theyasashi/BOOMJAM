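; BP_AbilityBase is the base class for abilities, defining activation, ending and event-response hooks for subclasses.
; Activate checks CanActivate, true by default, then passes the Target to OnActivate without storing it, since a reusable source can change targets.
; Initialize stores the Owner and registers the ability for each ListenTag with the GameInstance's GlobalBroadCastSubSystem.
; Broadcast forwards the tag, tag parameters and object to OnActivatedByEvent.
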(event Custom|EndAbility)

(event Custom|OnActivatedByEvent
  (params (Tag :type Gameplay%20Tag%20Structure) (TagParameters :type Gameplay%20Tag%20Container%20Structure) (Object :type Broadcast%20Parameter%20Base%20Object%20Reference)))

(event Custom|Activate
  (params (Target :type BP%20Target%20Info%20Base%20Object%20Reference))
  (bind __ (CallFunction|CanActivate Target))
  (if __
    (CallFunction|OnActivate Target)))

(event Custom|OnActivate
  (params (Target :type BP%20Target%20Info%20Base%20Object%20Reference)))

(event EventBroadcast
  (params (EventTag :type Gameplay%20Tag%20Structure) (标签参数 :type Gameplay%20Tag%20Container%20Structure) (对象参数 :type Broadcast%20Parameter%20Base%20Object%20Reference))
  (CallFunction|OnActivatedbyEvent EventTag 标签参数 对象参数))

(fn Initialize
  (params (Owner :type Actor%20Base%20Object%20Reference))
  (Variables|Default|SetOwner Owner)
  (bind _asbp_game_instance (Utilities|Casting|CastToBP_GameInstance (Game|GetGameInstance)))
  (for _array_element (GameplayTags|BreakGameplayTagContainer (Variables|Default|GetListenTags))
    (Default|监听Listen (Variables|/Game/Blueprints/Framework/BP_GameInstance.BP_GameInstance_C|GetGlobalBroadCastSubSystem _asbp_game_instance) _array_element self)))

(fn CanActivate
  (params (Target :type BP%20Target%20Info%20Base%20Object%20Reference))
  (return true))