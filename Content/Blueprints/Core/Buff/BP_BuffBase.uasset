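; Base buff that changes a target's float attributes using string formulas, with an activation check that passes by default.
; Modify fills each formula's variables from tagged attributes on the Source or Target, then writes the result to the Target's attribute.
; Compute is a hand-written expression evaluator that recursively resolves parentheses, then reduces multiply/divide and add/subtract by string substitution.
; A shared watchdog counter caps its loops.
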(fn Initialize
  (params (Source :type Actor%20Base%20Object%20Reference) (Target :type Actor%20Base%20Object%20Reference))
  (Variables|Default|SetSource Source)
  (Variables|Default|SetTarget Target))

(fn CanActivate
  (params (Target :type BP%20Target%20Info%20Base%20Object%20Reference))
  (return true))

(fn Modify
  (bind _target (Variables|Default|GetTarget))
  (for _array_element (Variables|Default|GetModifies)
    (LocalVariables|SetL_表达式 (Utilities|String|Replace (.计算式 (Utilities|Struct|BreakST_AttributeModifyDefine _array_element)) " "))
    (bind _keys (Utilities|Map|Keys (.Variables (Utilities|Struct|BreakST_AttributeModifyDefine _array_element))))
    (for _array_element_2 _keys
      (Utilities|IsValid (select (.FromTarget (Utilities|Struct|BreakST_AttributeVariableFloat (.Value (Utilities|Map|Find (.Variables (Utilities|Struct|BreakST_AttributeModifyDefine _array_element)) _array_element_2)))) (Variables|Default|GetTarget) (Variables|Default|GetSource))
        (:Is%20Valid
          (bind _attribute (Default|Get属性对象 (Variables|/Game/Blueprints/Core/ActorBase.ActorBase_C|GetAttributeComponent (select (.FromTarget (Utilities|Struct|BreakST_AttributeVariableFloat (.Value (Utilities|Map|Find (.Variables (Utilities|Struct|BreakST_AttributeModifyDefine _array_element)) _array_element_2)))) (Variables|Default|GetTarget) (Variables|Default|GetSource))) (.AttributeTag (Utilities|Struct|BreakST_AttributeVariableFloat (.Value (Utilities|Map|Find (.Variables (Utilities|Struct|BreakST_AttributeModifyDefine _array_element)) _array_element_2))))))
          (bind _asbp_attribute_base_float (Utilities|Casting|CastToBP_AttributeBase_Float _attribute))
          (bind _value (Default|GetValue _asbp_attribute_base_float (.FunctionTag (Utilities|Struct|BreakST_AttributeVariableFloat (.Value (Utilities|Map|Find (.Variables (Utilities|Struct|BreakST_AttributeModifyDefine _array_element)) _array_element_2))))))
          (Utilities|Map|Add (Variables|Default|GetVariablesValue) _array_element_2 _value))))
    (bind (_success _result) (CallFunction|Compute (LocalVariables|GetL_表达式) (Variables|Default|GetVariablesValue)))
    (if _success
      (Utilities|IsValid _target
        (:Is%20Valid
          (bind _attribute_2 (Default|Get属性对象 (Variables|/Game/Blueprints/Core/ActorBase.ActorBase_C|GetAttributeComponent _target) (.TargetAttribute (Utilities|Struct|BreakST_AttributeModifyDefine _array_element))))
          (bind _asbp_attribute_base_float_2 (Utilities|Casting|CastToBP_AttributeBase_Float _attribute_2))
          (Default|SetValue _asbp_attribute_base_float_2 (.TargetAttributeFunctionTag (Utilities|Struct|BreakST_AttributeModifyDefine _array_element)) _result))))))

(fn Compute
  (params (Expression :type String) (Variables :type Map%20of%20Strings%20to%20Float%20%28single-precision%29s))
  (bind _variablesvalue (Variables|Default|GetVariablesValue))
  (bind _variablesvalue_2 (Variables|Default|GetVariablesValue))
  (LocalVariables|SetL_Exp Expression)
  (Utilities|FlowControl|Sequence ; 1 括号\n2 乘除\n3 加减
    (:then_0
      (Utilities|FlowControl|Sequence
        (:then_0
          (LocalVariables|SetL_Start (Utilities|String|FindSubstring (LocalVariables|GetL_Exp) "(" false true) :!label _label)
          (if (>= (LocalVariables|GetL_Start) 0)
            (LocalVariables|SetL_End (Utilities|String|FindSubstring (LocalVariables|GetL_Exp) ")" false false (Utilities|String|FindSubstring (LocalVariables|GetL_Exp) "(" false true)))
            (if (> (LocalVariables|GetL_End) 0)
              (bind (_success _result) (CallFunction|Compute (Utilities|String|GetSubstring (LocalVariables|GetL_Exp) (+ (LocalVariables|GetL_Start) 1) (- (- (LocalVariables|GetL_End) (LocalVariables|GetL_Start)) 1)) Variables))
              (if _success
                (Development|PrintString (Utilities|String|Append (LocalVariables|GetL_Exp) "====>" (Utilities|String|Append (Utilities|String|SelectString (Utilities|String|Left (LocalVariables|GetL_Exp) (LocalVariables|GetL_Start)) "" (> (LocalVariables|GetL_Start) 0)) (Utilities|String|ToString(Float) _result) (Utilities|String|GetSubstring (LocalVariables|GetL_Exp) (+ (LocalVariables|GetL_End) 1) 2147483647))) false)
                (LocalVariables|SetL_Exp (Utilities|String|Append (Utilities|String|SelectString (Utilities|String|Left (LocalVariables|GetL_Exp) (LocalVariables|GetL_Start)) "" (> (LocalVariables|GetL_Start) 0)) (Utilities|String|ToString(Float) _result) (Utilities|String|GetSubstring (LocalVariables|GetL_Exp) (+ (LocalVariables|GetL_End) 1) 2147483647)))
                (bind _汪汪 (CallFunction|DogAdd))
                (if (not _汪汪)
                  (goto _label)))
              (else
                (return false 0.0) ; 括号不匹配
              ))))
        (:then_1
          (if (or (Utilities|String|Contains (LocalVariables|GetL_Exp) "(") (Utilities|String|Contains (LocalVariables|GetL_Exp) ")"))
            (return false 0.0) ; 括号不匹配
          ))))
    (:then_1
      (Utilities|FlowControl|Sequence
        (:then_0
          (bind _output_get (LocalVariables|SetL_运算符Index (Utilities|String|FindSubstring (LocalVariables|GetL_Exp) "*") :!label _label_2))
          (LocalVariables|SetL_ChengOrJia (> _output_get 0))
          (bind _output_get_2 (LocalVariables|SetL_ChuOrJian (Utilities|String|FindSubstring (LocalVariables|GetL_Exp) "/")))
          (if (and (> _output_get_2 0) (or (not (LocalVariables|GetL_ChengOrJia)) (< (LocalVariables|GetL_ChuOrJian) (LocalVariables|GetL_运算符Index))))
            (LocalVariables|SetL_运算符Index (LocalVariables|GetL_ChuOrJian))
            (LocalVariables|SetL_ChengOrJia false)
            (Utilities|FlowControl|Sequence :!label _label_3
              (:then_0
                (bind _output_get_3 (LocalVariables|SetL_Start (Math|Integer|Max(Integer) (Utilities|String|FindSubstring (Utilities|String|GetSubstring (LocalVariables|GetL_Exp) 0 (LocalVariables|GetL_运算符Index)) "+" false true) (Utilities|String|FindSubstring (Utilities|String|GetSubstring (LocalVariables|GetL_Exp) 0 (LocalVariables|GetL_运算符Index)) "-" false true) (Utilities|String|FindSubstring (Utilities|String|GetSubstring (LocalVariables|GetL_Exp) 0 (LocalVariables|GetL_运算符Index)) "*" false true) (Utilities|String|FindSubstring (Utilities|String|GetSubstring (LocalVariables|GetL_Exp) 0 (LocalVariables|GetL_运算符Index)) "/" false true))))
                (if (Math|Conversions|ToBoolean(Integer) _output_get_3)
                  (Math|Integer|IncrementInt (LocalVariables|GetL_Start)
                    (:%20%20
                      _)))
                (bind _output_get_4 (LocalVariables|SetL_VarLeft (Utilities|String|GetSubstring (LocalVariables|GetL_Exp) (LocalVariables|GetL_Start) (- (LocalVariables|GetL_运算符Index) (LocalVariables|GetL_Start)))))
                (if (.ReturnValue (Utilities|Map|Find _variablesvalue_2 _output_get_4))
                  (LocalVariables|SetL_VarValueLeft (.Value (Utilities|Map|Find _variablesvalue_2 _output_get_4)))
                  (elif (Class|KismetStringLibrary|IsNumeric _output_get_4)
                    (LocalVariables|SetL_VarValueLeft (Math|Conversions|ToFloat(Integer) _output_get_4))
                    (else
                      (return false 0.0)))))
              (:then_1
                (bind _output_get_5 (LocalVariables|SetL_End (Math|Integer|Max(Integer) (Math|Integer|Min(Integer) (Utilities|String|FindSubstring (Utilities|String|GetSubstring (LocalVariables|GetL_Exp) (+ (LocalVariables|GetL_运算符Index) 1) 2147483647) "+") (Utilities|String|FindSubstring (Utilities|String|GetSubstring (LocalVariables|GetL_Exp) (+ (LocalVariables|GetL_运算符Index) 1) 2147483647) "-") (Utilities|String|FindSubstring (Utilities|String|GetSubstring (LocalVariables|GetL_Exp) (+ (LocalVariables|GetL_运算符Index) 1) 2147483647) "*") (Utilities|String|FindSubstring (Utilities|String|GetSubstring (LocalVariables|GetL_Exp) (+ (LocalVariables|GetL_运算符Index) 1) 2147483647) "/")))))
                (if (Math|Conversions|ToBoolean(Integer) _output_get_5)
                  _
                  (else
                    (LocalVariables|SetL_End (Utilities|String|Len (LocalVariables|GetL_Exp)))))
                (bind _output_get_6 (LocalVariables|SetL_VarRight (Utilities|String|GetSubstring (LocalVariables|GetL_Exp) (+ (LocalVariables|GetL_运算符Index) 1) (- (LocalVariables|GetL_End) (+ (LocalVariables|GetL_运算符Index) 1)))))
                (if (.ReturnValue (Utilities|Map|Find _variablesvalue_2 _output_get_6))
                  (LocalVariables|SetL_VarValueRight (.Value (Utilities|Map|Find _variablesvalue_2 _output_get_6)))
                  (elif (Class|KismetStringLibrary|IsNumeric _output_get_6)
                    (LocalVariables|SetL_VarValueRight (Math|Conversions|ToFloat(Integer) _output_get_6))
                    (else
                      (return false 0.0)))))
              (:then_2
                (if (LocalVariables|GetL_ChengOrJia)
                  (LocalVariables|SetL_Exp (Utilities|String|Append (Utilities|String|GetSubstring (LocalVariables|GetL_Exp) 0 (LocalVariables|GetL_Start)) (Utilities|String|ToString(Float) (* (LocalVariables|GetL_VarValueLeft) (LocalVariables|GetL_VarValueRight))) (Utilities|String|GetSubstring (LocalVariables|GetL_Exp) (LocalVariables|GetL_End) 2147483647)))
                  (else
                    (LocalVariables|SetL_Exp (Utilities|String|Append (Utilities|String|GetSubstring (LocalVariables|GetL_Exp) 0 (LocalVariables|GetL_Start)) (Utilities|String|ToString(Float) (/ (LocalVariables|GetL_VarValueLeft) (LocalVariables|GetL_VarValueRight))) (Utilities|String|GetSubstring (LocalVariables|GetL_Exp) (LocalVariables|GetL_End) 2147483647)))))
                (bind _汪汪_2 (CallFunction|DogAdd))
                (if (not _汪汪_2)
                  (goto _label_2))))
            (elif (LocalVariables|GetL_ChengOrJia)
              (goto _label_3))))
        (:then_1
          (if (or (Utilities|String|Contains (LocalVariables|GetL_Exp) "*") (Utilities|String|Contains (LocalVariables|GetL_Exp) "/"))
            (return false 0.0)))))
    (:then_2
      (bind _output_get_7 (LocalVariables|SetL_运算符Index (Utilities|String|FindSubstring (LocalVariables|GetL_Exp) "+") :!label _label_4))
      (LocalVariables|SetL_ChengOrJia (> _output_get_7 0))
      (bind _output_get_8 (LocalVariables|SetL_ChuOrJian (Utilities|String|FindSubstring (LocalVariables|GetL_Exp) "-")))
      (if (and (> _output_get_8 0) (or (not (LocalVariables|GetL_ChengOrJia)) (< (LocalVariables|GetL_ChuOrJian) (LocalVariables|GetL_运算符Index))))
        (LocalVariables|SetL_运算符Index (LocalVariables|GetL_ChuOrJian))
        (LocalVariables|SetL_ChengOrJia false)
        (Utilities|FlowControl|Sequence :!label _label_5
          (:then_0
            (LocalVariables|SetL_Start 0)
            (bind _output_get_9 (LocalVariables|SetL_VarLeft (Utilities|String|GetSubstring (LocalVariables|GetL_Exp) 0 (LocalVariables|GetL_运算符Index))))
            (if (.ReturnValue (Utilities|Map|Find _variablesvalue _output_get_9))
              (LocalVariables|SetL_VarValueLeft (.Value (Utilities|Map|Find _variablesvalue _output_get_9)))
              (elif (Class|KismetStringLibrary|IsNumeric _output_get_9)
                (LocalVariables|SetL_VarValueLeft (Math|Conversions|ToFloat(Integer) _output_get_9))
                (else
                  (return false 0.0)))))
          (:then_1
            (bind _output_get_10 (LocalVariables|SetL_End (Math|Integer|Max(Integer) (Math|Integer|Min(Integer) (Utilities|String|FindSubstring (Utilities|String|GetSubstring (LocalVariables|GetL_Exp) (+ (LocalVariables|GetL_运算符Index) 1) 2147483647) "+") (Utilities|String|FindSubstring (Utilities|String|GetSubstring (LocalVariables|GetL_Exp) (+ (LocalVariables|GetL_运算符Index) 1) 2147483647) "-")))))
            (if (Math|Conversions|ToBoolean(Integer) _output_get_10)
              _
              (else
                (LocalVariables|SetL_End (Utilities|String|Len (LocalVariables|GetL_Exp)))))
            (bind _output_get_11 (LocalVariables|SetL_VarRight (Utilities|String|GetSubstring (LocalVariables|GetL_Exp) (+ (LocalVariables|GetL_运算符Index) 1) (- (LocalVariables|GetL_End) (+ (LocalVariables|GetL_运算符Index) 1)))))
            (if (.ReturnValue (Utilities|Map|Find _variablesvalue _output_get_11))
              (LocalVariables|SetL_VarValueRight (.Value (Utilities|Map|Find _variablesvalue _output_get_11)))
              (elif (Class|KismetStringLibrary|IsNumeric _output_get_11)
                (LocalVariables|SetL_VarValueRight (Math|Conversions|ToFloat(Integer) _output_get_11))
                (else
                  (return false 0.0)))))
          (:then_2
            (if (LocalVariables|GetL_ChengOrJia)
              (LocalVariables|SetL_Exp (Utilities|String|Append (Utilities|String|GetSubstring (LocalVariables|GetL_Exp) 0 (LocalVariables|GetL_Start)) (Utilities|String|ToString(Float) (+ (LocalVariables|GetL_VarValueLeft) (LocalVariables|GetL_VarValueRight))) (Utilities|String|GetSubstring (LocalVariables|GetL_Exp) (LocalVariables|GetL_End) 2147483647)))
              (else
                (LocalVariables|SetL_Exp (Utilities|String|Append (Utilities|String|GetSubstring (LocalVariables|GetL_Exp) 0 (LocalVariables|GetL_Start)) (Utilities|String|ToString(Float) (- (LocalVariables|GetL_VarValueLeft) (LocalVariables|GetL_VarValueRight))) (Utilities|String|GetSubstring (LocalVariables|GetL_Exp) (LocalVariables|GetL_End) 2147483647)))))
            (bind _汪汪_3 (CallFunction|DogAdd))
            (if (not _汪汪_3)
              (goto _label_4))))
        (elif (LocalVariables|GetL_ChengOrJia)
          (goto _label_5))))
    (:then_3
      (return (Class|KismetStringLibrary|IsNumeric (LocalVariables|GetL_Exp)) (Math|Conversions|ToFloat(Integer) (LocalVariables|GetL_Exp))))))

(fn DogAdd
  (bind _result (Math|Integer|IncrementInt (Variables|Default|GetDogCount))
    (:%20%20
      (return (> _result 100)))))