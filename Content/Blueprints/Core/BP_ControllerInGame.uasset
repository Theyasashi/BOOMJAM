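; In-game player controller for a hex-tile game, handling top-down camera movement, tile selection and the HUD.
; Move axes pan the pawn, while Tick eases spring arm length toward Viewheight and glides the pawn to the last clicked point.
; Clicking a grass hex selects any player actor on it in the game state, or draws a debug sphere if empty.
; The selected actor's actions for that tile then fill the HUD action list.
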(event EventBeginPlay
  (|CallParentFunction)
  (Input|SetInputModeGameandUI self 0 "DoNotLock" true)
  (Variables|Default|SetbShowMouseCursor true)
  (bind _returnvalue (UserInterface|CreateWidget "/Game/Blueprints/UI/WBP_HUD.WBP_HUD_C" self))
  (bind _output_get (Variables|Default|SetHUD _returnvalue))
  (UserInterface|Viewport|AddtoViewport _output_get 0)
  (bind _astop_down_character (Utilities|Casting|CastToTopDownCharacter (Pawn|GetControlledPawn)))
  (Variables|Default|SetSpringArm (Variables|/Game/TopDownBP/Blueprints/TopDownCharacter.TopDownCharacter_C|GetSpringArm1 _astop_down_character)))

(event EventTick
  (params (DeltaSeconds :type Float%20%28single-precision%29))
  (bind _returnvalue (Pawn|GetControlledPawn))
  (bind _viewmovelocation (Variables|Default|GetViewMoveLocation))
  (bind _springarm (Variables|Default|GetSpringArm))
  (bind _returnvalue_2 (Transformation|GetActorLocation _returnvalue))
  (|CallParentFunction DeltaSeconds)
  (Variables|/Script/Engine.SpringArmComponent|SetTargetArmLength _springarm (Math|Float|Lerp (Variables|/Script/Engine.SpringArmComponent|GetTargetArmLength _springarm) (* (Variables|Default|GetViewheight) 1e+02) 0.1))
  (if (Variables|Default|GetViewQuickMoving)
    (Transformation|SetActorLocation (Pawn|GetControlledPawn) (Math|Vector|Lerp(Vector) _returnvalue_2 _viewmovelocation 0.5) false false)
    (if (Math|Vector|Equal(Vector) _returnvalue_2 _viewmovelocation 1.0)
      (Variables|Default|SetViewQuickMoving false))))

(event Input|ActionEvents|InputActionSetDestination
  (params (Key :type Key%20Structure :default "None"))
  (bind _hitresult (Game|Player|GetHitResultUnderCursorbyChannel "TraceTypeQuery1" true))
  (bind (_bblockinghit _binitialoverlap _time _distance _location _impactpoint _normal _impactnormal _physmat _hitactor) (Collision|BreakHitResult _hitresult))
  (:Pressed
    (Variables|Default|SetViewMoveLocation (Math|Vector|MakeVector (.x _location) (.y _location) (.z (Transformation|GetActorLocation (Pawn|GetControlledPawn)))))
    (Variables|Default|SetViewQuickMoving true)
    (bind _asbp_hex_tile_grass (Utilities|Casting|CastToBp_HexTile_Grass _hitactor))
    (Variables|Default|SetLastSelectedTile _asbp_hex_tile_grass)
    (Utilities|FlowControl|Sequence
      (:then_0
        (Utilities|IsValid (Variables|/Game/SqrSLG/Blueprints/Bp_HexTile_Grass.Bp_HexTile_Grass_C|GetActorOnHexTile _asbp_hex_tile_grass)
          (:Is%20Valid
            (Utilities|Casting|CastToPlayerActorBase (Variables|/Game/SqrSLG/Blueprints/Bp_HexTile_Grass.Bp_HexTile_Grass_C|GetActorOnHexTile _asbp_hex_tile_grass))
            (Variables|/Game/Blueprints/Framework/BP_GameStateInGame.BP_GameStateInGame_C|SetSelectedActor (.AsBP%20Game%20State%20in%20Game (Utilities|Casting|CastToBP_GameStateInGame (Game|GetGameState))) (Variables|/Game/SqrSLG/Blueprints/Bp_HexTile_Grass.Bp_HexTile_Grass_C|GetActorOnHexTile _asbp_hex_tile_grass)))
          (:Is%20Not%20Valid
            (Rendering|Debug|DrawDebugSphere (Transformation|GetActorLocation _asbp_hex_tile_grass) 2e+01 12 "(R=1.000000,G=0.000000,B=0.241171,A=1.000000)" 1e+01 2.0))))
      (:then_1
        (bind _asplayer_actor_base (Utilities|Casting|CastToPlayerActorBase (Variables|/Game/Blueprints/Framework/BP_GameStateInGame.BP_GameStateInGame_C|GetSelectedActor (.AsBP%20Game%20State%20in%20Game (Utilities|Casting|CastToBP_GameStateInGame (Game|GetGameState))))))
        (bind _tags (Default|GetActions _asplayer_actor_base _asbp_hex_tile_grass))
        (Default|UpdateActionList (Variables|Default|GetHUD) _tags)))))

(event Input|AxisEvents|InputAxisMoveForward
  (params (AxisValue :type Float%20%28single-precision%29))
  (if (not (Variables|Default|GetViewQuickMoving))
    (Pawn|Input|AddMovementInput (Pawn|GetControlledPawn) (Math|Vector|MakeVector (* AxisValue (Utilities|Time|GetWorldDeltaSeconds) 6e+02) 0.0 0.0) 1.0 false)))

(event Input|AxisEvents|InputAxisMoveRight
  (params (AxisValue :type Float%20%28single-precision%29))
  (if (not (Variables|Default|GetViewQuickMoving))
    (Pawn|Input|AddMovementInput (Pawn|GetControlledPawn) (Math|Vector|MakeVector 0.0 (* AxisValue (Utilities|Time|GetWorldDeltaSeconds) 6e+02) 0.0) 1.0 false)))

(fn ConstructionScript)