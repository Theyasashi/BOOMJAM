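; Base attribute object identified by a gameplay tag, holding a current value plus tag-keyed function values such as Max and Min for an owner.
; Initialize takes values from the save game if Save-tagged, else from curve tables named after the attribute, by owner name and level, then clamps.
; SetValue broadcasts change events through a reused parameter object without clamping; Initialize forces an initial event.
; Save persists values per owner ID.
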(fn GetValue
  (params (FunctionTag :type Gameplay%20Tag%20Structure))
  (if (or (not (GameplayTags|IsGameplayTagValid FunctionTag)) (== (Variables|Default|GetTag) FunctionTag))
    (return (Variables|Default|GetCurrent))
    (else
      (return (.Value (Utilities|Map|Find (Variables|Default|GetFunctionValue) FunctionTag))))))

(fn SetValue
  (params (FunctionTag :type Gameplay%20Tag%20Structure) (NewValue :type Float%20%28single-precision%29))
  (bind _globalbroadcastsubsystem (|Broadcast))
  (bind _functionvalue (Variables|Default|GetFunctionValue))
  (bind _onvaluechangeparameter (Variables|Default|GetOnValueChangeParameter))
  (bind _onvaluechangeparameter_2 (Variables|Default|GetOnValueChangeParameter))
  (bind _attributename (Variables|Default|GetAttributeName))
  (bind (_value _returnvalue) (Utilities|Map|Find _functionvalue FunctionTag))
  (bind _returnvalue_2 (Utilities|String|Append "Attribute." _attributename ".Event.Change"))
  (if (or (not (GameplayTags|IsGameplayTagValid FunctionTag)) (== (Variables|Default|GetTag) FunctionTag))
    (if (!= (Variables|Default|GetCurrent) NewValue)
      (Default|Init _onvaluechangeparameter_2 (Variables|Default|GetOwner) (Variables|Default|GetCurrent) NewValue)
      (Variables|Default|SetCurrent NewValue)
      (bind _returnvalue_3 (Class|MyBlueprintFunctionLibrary|MakeGameplayTagfromString _returnvalue_2))
      (Default|广播Broadcast _globalbroadcastsubsystem _returnvalue_3 "(GameplayTags=)" _onvaluechangeparameter_2))
    (elif _returnvalue
      (Default|Init _onvaluechangeparameter (Variables|Default|GetOwner) _value NewValue)
      (Utilities|Map|Add _functionvalue FunctionTag NewValue)
      (bind _returnvalue_4 (Class|MyBlueprintFunctionLibrary|MakeGameplayTagfromString _returnvalue_2))
      (Default|广播Broadcast _globalbroadcastsubsystem _returnvalue_4 (GameplayTags|MakeGameplayTagContainerfromTag FunctionTag) _onvaluechangeparameter))))

(fn Initialize
  (params (Owner :type Actor%20Base%20Object%20Reference))
  (bind _output_get (Variables|Default|SetOwner Owner))
  (bind _returnvalue (Game|ConstructObjectfromClass "/Game/Blueprints/Core/Attribute/BP_OnAttributeValueChangeParameter.BP_OnAttributeValueChangeParameter_C" _output_get))
  (Variables|Default|SetOnValueChangeParameter _returnvalue)
  (Variables|Default|SetAttributeName (CallFunction|GetCurveTableName))
  (LocalVariables|SetL_Save (Variables|/Game/Blueprints/Framework/BP_GameInstance.BP_GameInstance_C|GetSaveGameInstance (.AsBP%20Game%20Instance (Utilities|Casting|CastToBP_GameInstance (Game|GetGameInstance)))))
  (Utilities|FlowControl|Sequence
    (:then_0
      (bind _output_get_2 (LocalVariables|SetHasSave (GameplayTags|HasTag (Variables|Default|GetTags) "(TagName=\"Attribute.Function.Save\")" true)))
      (if _output_get_2
        (bind (_value _has) (Default|GetFloat (LocalVariables|GetL_Save) (Variables|/Game/Blueprints/Core/ActorBase.ActorBase_C|GetId (Variables|Default|GetOwner)) (GameplayTags|GetTagName (Variables|Default|GetTag))))
        (if _has
          (LocalVariables|SetL_CurrentValue _value)
          (else
            (bind _returnvalue_2 (Class|MyBlueprintFunctionLibrary|LoadCurveTable (Utilities|MakeSoftObjectPath (Utilities|String|Append (Variables|Default|GetAttributesRoot) (Variables|Default|GetAttributeName))) :!label _label))
            (bind _outxy (DataTable|EvaluateCurveTableRow _returnvalue_2 (Variables|/Game/Blueprints/Core/ActorBase.ActorBase_C|GetName (Variables|Default|GetOwner)) (Math|Conversions|ToFloat(Integer) (Variables|/Game/Blueprints/Core/ActorBase.ActorBase_C|GetLevel (Variables|Default|GetOwner))))
              (:RowFound
                (LocalVariables|SetL_CurrentValue _outxy))
              (:RowNotFound
                (return)))))
        (else
          (goto _label))))
    (:then_1
      (if (GameplayTags|HasTag (Variables|Default|GetTags) "(TagName=\"Attribute.Function.Max\")" true) ; 最大值限制
        (if (LocalVariables|GetHasSave)
          (bind (_value_2 _has_2) (Default|GetFloat (LocalVariables|GetL_Save) (Variables|/Game/Blueprints/Core/ActorBase.ActorBase_C|GetId (Variables|Default|GetOwner)) (Utilities|String|StringToName (Utilities|String|Append (GameplayTags|GetDebugStringfromGameplayTag (Variables|Default|GetTag)) "+" (GameplayTags|GetDebugStringfromGameplayTag "(TagName=\"Attribute.Function.Max\")")))))
          (if _has_2
            (LocalVariables|SetL_MaxValue _value_2)
            (else
              (bind _returnvalue_3 (Class|MyBlueprintFunctionLibrary|LoadCurveTable (Utilities|MakeSoftObjectPath (Utilities|String|Append (Variables|Default|GetAttributesRoot) (Variables|Default|GetAttributeName) "Max")) :!label _label_2))
              (bind _outxy_2 (DataTable|EvaluateCurveTableRow _returnvalue_3 (Variables|/Game/Blueprints/Core/ActorBase.ActorBase_C|GetName (Variables|Default|GetOwner)) (Math|Conversions|ToFloat(Integer) (Variables|/Game/Blueprints/Core/ActorBase.ActorBase_C|GetLevel (Variables|Default|GetOwner))))
                (:RowFound
                  (LocalVariables|SetL_MaxValue _outxy_2)))))
          (else
            (goto _label_2)))
        (LocalVariables|SetL_CurrentValue (Math|Float|Min(Float) (LocalVariables|GetL_CurrentValue) (LocalVariables|GetL_MaxValue)))
        (Utilities|Map|Add (Variables|Default|GetFunctionValue) "(TagName=\"Attribute.Function.Max\")" (LocalVariables|GetL_MaxValue))))
    (:then_2
      (if (GameplayTags|HasTag (Variables|Default|GetTags) "(TagName=\"Attribute.Function.Min\")" true) ; 最小值限制
        (if (LocalVariables|GetHasSave)
          (bind (_value_3 _has_3) (Default|GetFloat (LocalVariables|GetL_Save) (Variables|/Game/Blueprints/Core/ActorBase.ActorBase_C|GetId (Variables|Default|GetOwner)) (Utilities|String|StringToName (Utilities|String|Append (GameplayTags|GetDebugStringfromGameplayTag (Variables|Default|GetTag)) "+" (GameplayTags|GetDebugStringfromGameplayTag "(TagName=\"Attribute.Function.Min\")")))))
          (if _has_3
            (LocalVariables|SetL_MinValue _value_3)
            (else
              (bind _returnvalue_4 (Class|MyBlueprintFunctionLibrary|LoadCurveTable (Utilities|MakeSoftObjectPath (Utilities|String|Append (Variables|Default|GetAttributesRoot) (Variables|Default|GetAttributeName) "Min")) :!label _label_3))
              (bind _outxy_3 (DataTable|EvaluateCurveTableRow _returnvalue_4 (Variables|/Game/Blueprints/Core/ActorBase.ActorBase_C|GetName (Variables|Default|GetOwner)) (Math|Conversions|ToFloat(Integer) (Variables|/Game/Blueprints/Core/ActorBase.ActorBase_C|GetLevel (Variables|Default|GetOwner))))
                (:RowFound
                  (LocalVariables|SetL_MinValue _outxy_3)))))
          (else
            (goto _label_3)))
        (LocalVariables|SetL_CurrentValue (Math|Float|Max(Float) (LocalVariables|GetL_CurrentValue) (LocalVariables|GetL_MinValue)))
        (Utilities|Map|Add (Variables|Default|GetFunctionValue) "(TagName=\"Attribute.Function.Min\")" (LocalVariables|GetL_MinValue))))
    (:then_3
      (Variables|Default|SetCurrent (- (LocalVariables|GetL_CurrentValue) 1.0)) ; 故意设置不同值，以便触发变更事件
      (CallFunction|SetValue :NewValue (LocalVariables|GetL_CurrentValue)))))

(fn GetCurveTableName
  (bind _tag (Variables|Default|GetTag))
  (bind _returnvalue (GameplayTags|GetDebugStringfromGameplayTag _tag))
  (return (Utilities|String|GetSubstring _returnvalue (+ (Utilities|String|FindSubstring _returnvalue "." false true) 1) (Utilities|String|Len _returnvalue))))

(fn Save
  (bind _returnvalue (Game|GetGameInstance))
  (bind _functionvalue (Variables|Default|GetFunctionValue))
  (bind _owner (Variables|Default|GetOwner))
  (bind _asbp_game_instance (Utilities|Casting|CastToBP_GameInstance _returnvalue))
  (bind _id (Variables|/Game/Blueprints/Core/ActorBase.ActorBase_C|GetId _owner))
  (bind _savegameinstance (Variables|/Game/Blueprints/Framework/BP_GameInstance.BP_GameInstance_C|GetSaveGameInstance _asbp_game_instance))
  (if (GameplayTags|HasTag (Variables|Default|GetTags) "(TagName=\"Attribute.Function.Save\")" true)
    (Default|ModifyFloat _savegameinstance _id (GameplayTags|GetTagName (Variables|Default|GetTag)) (Variables|Default|GetCurrent) false)
    (bind _keys (Utilities|Map|Keys _functionvalue))
    (for _array_element _keys
      (Default|ModifyFloat _savegameinstance _id (Utilities|String|StringToName (Utilities|String|Append (GameplayTags|GetDebugStringfromGameplayTag (Variables|Default|GetTag)) "+" (GameplayTags|GetDebugStringfromGameplayTag _array_element))) (.Value (Utilities|Map|Find _functionvalue _array_element)) false))))