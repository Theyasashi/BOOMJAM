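; General base attribute Blueprint, identified by a gameplay tag and tied to an owner.
; Initialize stores the owner and sets AttributeName from GetCurveTableName, which takes the tag text after its last dot.
; The function name suggests this short name serves as a curve table key, though no lookup happens here.
; Save is an empty stub.
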(fn Initialize
  (params (Owner :type Actor%20Base%20Object%20Reference))
  (Variables|Default|SetOwner Owner)
  (Variables|Default|SetAttributeName (CallFunction|GetCurveTableName)))

(fn GetCurveTableName
  (bind _tag (Variables|Default|GetTag))
  (bind _returnvalue (GameplayTags|GetDebugStringfromGameplayTag _tag))
  (return (Utilities|String|GetSubstring _returnvalue (+ (Utilities|String|FindSubstring _returnvalue "." false true) 1) (Utilities|String|Len _returnvalue))))

(fn Save)