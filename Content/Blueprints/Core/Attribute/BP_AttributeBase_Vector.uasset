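; Vector attribute for an owner object, holding a current value plus sub-values keyed by function gameplay tag.
; SetValue raises attribute-change events through a reusable parameter object, though the sub-value branch re-stores the old value.
; Save-tagged attributes write to the GameInstance's save object by owner ID and tag name.
; Initialize reads the saved value, offsets Current from it, then sets zero to trigger a change event.
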(fn GetValue
  (params (FunctionTag :type Gameplay%20Tag%20Structure))
  (if (or (not (GameplayTags|IsGameplayTagValid FunctionTag)) (== (Variables|Default|GetTag) FunctionTag))
    (return (Variables|Default|GetCurrent))
    (else
      (return (.Value (Utilities|Map|Find (Variables|Default|GetFunctionValue) FunctionTag))))))

(fn SetValue
  (params (FunctionTag :type Gameplay%20Tag%20Structure) (NewValue :type Vector))
  (bind _functionvalue (Variables|Default|GetFunctionValue))
  (bind _onvaluechangeparameter (Variables|Default|GetOnValueChangeParameter))
  (bind _owner (Variables|Default|GetOwner))
  (bind (_value _returnvalue) (Utilities|Map|Find _functionvalue FunctionTag))
  (LocalVariables|SetL_New NewValue)
  (if (or (not (GameplayTags|IsGameplayTagValid FunctionTag)) (== (Variables|Default|GetTag) FunctionTag))
    (if (Math|Vector|NotEqual(Vector) (Variables|Default|GetCurrent) (LocalVariables|GetL_New) 0.1)
      (Default|Init _onvaluechangeparameter _owner (Variables|Default|GetCurrent) (LocalVariables|GetL_New))
      (Variables|Default|SetCurrent (LocalVariables|GetL_New))
      (Default|CallOnAttributeChanged :AttributeTag (Variables|Default|GetTag) :Parameter _onvaluechangeparameter))
    (elif _returnvalue
      (Default|Init _onvaluechangeparameter _owner _value (LocalVariables|GetL_New))
      (Utilities|Map|Add _functionvalue FunctionTag _value)
      (Default|CallOnAttributeChanged (Variables|Default|GetTag) FunctionTag _onvaluechangeparameter))))

(fn Save
  (bind _returnvalue (Game|GetGameInstance))
  (bind _functionvalue (Variables|Default|GetFunctionValue))
  (bind _owner (Variables|Default|GetOwner))
  (bind _asbp_game_instance (Utilities|Casting|CastToBP_GameInstance _returnvalue))
  (bind _id (Variables|/Game/Blueprints/Core/ActorBase.ActorBase_C|GetId _owner))
  (bind _savegameinstance (Variables|/Game/Blueprints/Framework/BP_GameInstance.BP_GameInstance_C|GetSaveGameInstance _asbp_game_instance))
  (|CallParentFunction)
  (if (GameplayTags|HasTag (Variables|Default|GetTags) "(TagName=\"Attribute.Function.Save\")" true)
    (Default|ModifyVector _savegameinstance _id (GameplayTags|GetTagName (Variables|Default|GetTag)) (Variables|Default|GetCurrent) false)
    (bind _keys (Utilities|Map|Keys _functionvalue))
    (for _array_element _keys
      (Default|ModifyVector _savegameinstance _id (Utilities|String|StringToName (Utilities|String|Append (GameplayTags|GetDebugStringfromGameplayTag (Variables|Default|GetTag)) "+" (GameplayTags|GetDebugStringfromGameplayTag _array_element))) (.Value (Utilities|Map|Find _functionvalue _array_element)) false))))

(fn Initialize
  (params (Owner :type Actor%20Base%20Object%20Reference))
  (|CallParentFunction Owner)
  (LocalVariables|SetL_Save (Variables|/Game/Blueprints/Framework/BP_GameInstance.BP_GameInstance_C|GetSaveGameInstance (.AsBP%20Game%20Instance (Utilities|Casting|CastToBP_GameInstance (Game|GetGameInstance)))))
  (bind _returnvalue (Game|ConstructObjectfromClass "/Game/Blueprints/Core/Attribute/BP_OnAttributeValueChangeParameter_Vector.BP_OnAttributeValueChangeParameter_Vector_C" (Variables|Default|GetOwner)))
  (Variables|Default|SetOnValueChangeParameter _returnvalue)
  (Utilities|FlowControl|Sequence
    (:then_0
      (bind _output_get (LocalVariables|SetL_HasSave (GameplayTags|HasTag (Variables|Default|GetTags) "(TagName=\"Attribute.Function.Save\")" true)))
      (if _output_get
        (bind (_value _has) (Default|GetVector (LocalVariables|GetL_Save) (Variables|/Game/Blueprints/Core/ActorBase.ActorBase_C|GetId (Variables|Default|GetOwner)) (GameplayTags|GetTagName (Variables|Default|GetTag))))
        (if _has
          (LocalVariables|SetL_CurrentValue _value)
          (else
            (return)))
        (else
          (return))))
    (:then_1
      (Variables|Default|SetCurrent (- (LocalVariables|GetL_CurrentValue) 1)) ; 故意设置不同值，以便触发变更事件
      (CallFunction|SetValue))))