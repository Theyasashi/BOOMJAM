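; Base float attribute for an owner, holding a current value plus tag-keyed function values such as Max and Min.
; Initialize restores save-flagged values, falling back to curve tables by owner name and level.
; SetValue clamps the current value, non-negative by default without a Min, and broadcasts changes; Save writes flagged values per owner ID.
; Initialize deliberately offsets Current before SetValue to force an initial change event.
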(fn GetValue
  (params (FunctionTag :type Gameplay%20Tag%20Structure))
  (if (or (not (GameplayTags|IsGameplayTagValid FunctionTag)) (== (Variables|Default|GetTag) FunctionTag))
    (return (Variables|Default|GetCurrent))
    (else
      (return (.Value (Utilities|Map|Find (Variables|Default|GetFunctionValue) FunctionTag))))))

(fn SetValue
  (params (FunctionTag :type Gameplay%20Tag%20Structure) (NewValue :type Float%20%28single-precision%29))
  (bind _globalbroadcastsubsystem (|Broadcast))
  (bind _functionvalue (Variables|Default|GetFunctionValue))
  (bind _onvaluechangeparameter (Variables|Default|GetOnValueChangeParameter))
  (bind _onvaluechangeparameter_2 (Variables|Default|GetOnValueChangeParameter))
  (bind _attributesroot (Variables|Default|GetAttributesRoot))
  (bind (_value _returnvalue) (Utilities|Map|Find _functionvalue FunctionTag))
  (bind _returnvalue_2 (Utilities|String|Append "Attribute." _attributesroot ".Event.Change"))
  (LocalVariables|SetL_New NewValue)
  (if (or (not (GameplayTags|IsGameplayTagValid FunctionTag)) (== (Variables|Default|GetTag) FunctionTag))
    (bind _约束 (CallFunction|LimitValue (LocalVariables|GetL_New)))
    (LocalVariables|SetL_New _约束)
    (if (!= (Variables|Default|GetCurrent) (LocalVariables|GetL_New))
      (Default|Init _onvaluechangeparameter_2 (Variables|Default|GetOwner) (Variables|Default|GetCurrent) (LocalVariables|GetL_New))
      (Variables|Default|SetCurrent (LocalVariables|GetL_New))
      (bind _returnvalue_3 (Class|MyBlueprintFunctionLibrary|MakeGameplayTagfromString _returnvalue_2))
      (if (GameplayTags|IsGameplayTagValid _returnvalue_3)
        (Default|广播Broadcast _globalbroadcastsubsystem _returnvalue_3 "(GameplayTags=)" _onvaluechangeparameter_2)
        (Default|CallOnAttributeChanged :AttributeTag (Variables|Default|GetTag) :Parameter _onvaluechangeparameter_2)))
    (elif _returnvalue
      (Default|Init _onvaluechangeparameter (Variables|Default|GetOwner) _value (LocalVariables|GetL_New))
      (Utilities|Map|Add _functionvalue FunctionTag (LocalVariables|GetL_New))
      (bind _returnvalue_4 (Class|MyBlueprintFunctionLibrary|MakeGameplayTagfromString _returnvalue_2))
      (if (GameplayTags|IsGameplayTagValid _returnvalue_4)
        (Default|广播Broadcast _globalbroadcastsubsystem _returnvalue_4 (GameplayTags|MakeGameplayTagContainerfromTag FunctionTag) _onvaluechangeparameter)
        (Default|CallOnAttributeChanged (Variables|Default|GetTag) FunctionTag _onvaluechangeparameter)))))

(fn LimitValue
  (params (原值 :type Float%20%28single-precision%29))
  (bind _functionvalue (Variables|Default|GetFunctionValue))
  (bind (_value _returnvalue) (Utilities|Map|Find _functionvalue "(TagName=\"Attribute.Function.Min\")"))
  (bind (_value_2 _returnvalue_2) (Utilities|Map|Find _functionvalue "(TagName=\"Attribute.Function.Max\")"))
  (LocalVariables|SetL_Origin 原值)
  (Utilities|FlowControl|Sequence
    (:then_0
      (if _returnvalue_2
        (LocalVariables|SetL_Origin (Math|Float|Min(Float) (LocalVariables|GetL_Origin) _value_2))))
    (:then_1
      (if _returnvalue
        (LocalVariables|SetL_Origin (Math|Float|Max(Float) (LocalVariables|GetL_Origin) _value))
        (elif (and (< (LocalVariables|GetL_Origin) 0.0) (not (GameplayTags|HasTag (Variables|Default|GetTags) "(TagName=\"Attribute.Function.CanNegative\")" true)))
          (LocalVariables|SetL_Origin 0.0))))
    (:then_2
      (return (LocalVariables|GetL_Origin)))))

(fn Save
  (bind _returnvalue (Game|GetGameInstance))
  (bind _functionvalue (Variables|Default|GetFunctionValue))
  (bind _owner (Variables|Default|GetOwner))
  (bind _asbp_game_instance (Utilities|Casting|CastToBP_GameInstance _returnvalue))
  (bind _id (Variables|/Game/Blueprints/Core/ActorBase.ActorBase_C|GetId _owner))
  (bind _savegameinstance (Variables|/Game/Blueprints/Framework/BP_GameInstance.BP_GameInstance_C|GetSaveGameInstance _asbp_game_instance))
  (|CallParentFunction)
  (if (GameplayTags|HasTag (Variables|Default|GetTags) "(TagName=\"Attribute.Function.Save\")" true)
    (Default|ModifyFloat _savegameinstance _id (GameplayTags|GetTagName (Variables|Default|GetTag)) (Variables|Default|GetCurrent) false)
    (bind _keys (Utilities|Map|Keys _functionvalue))
    (for _array_element _keys
      (Default|ModifyFloat _savegameinstance _id (Utilities|String|StringToName (Utilities|String|Append (GameplayTags|GetDebugStringfromGameplayTag (Variables|Default|GetTag)) "+" (GameplayTags|GetDebugStringfromGameplayTag _array_element))) (.Value (Utilities|Map|Find _functionvalue _array_element)) false))))

(fn Initialize
  (params (Owner :type Actor%20Base%20Object%20Reference))
  (|CallParentFunction Owner)
  (bind _returnvalue (Game|ConstructObjectfromClass "/Game/Blueprints/Core/Attribute/BP_OnAttributeValueChangeParameter_Float.BP_OnAttributeValueChangeParameter_Float_C" (Variables|Default|GetOwner)))
  (Variables|Default|SetOnValueChangeParameter _returnvalue)
  (LocalVariables|SetL_Save (Variables|/Game/Blueprints/Framework/BP_GameInstance.BP_GameInstance_C|GetSaveGameInstance (.AsBP%20Game%20Instance (Utilities|Casting|CastToBP_GameInstance (Game|GetGameInstance)))))
  (Utilities|FlowControl|Sequence
    (:then_0
      (bind _output_get (LocalVariables|SetL_HasSave (GameplayTags|HasTag (Variables|Default|GetTags) "(TagName=\"Attribute.Function.Save\")" true)))
      (if _output_get
        (bind (_value _has) (Default|GetFloat (LocalVariables|GetL_Save) (Variables|/Game/Blueprints/Core/ActorBase.ActorBase_C|GetId (Variables|Default|GetOwner)) (GameplayTags|GetTagName (Variables|Default|GetTag))))
        (if _has
          (LocalVariables|SetL_CurrentValue _value)
          (else
            (bind _returnvalue_2 (Class|MyBlueprintFunctionLibrary|LoadCurveTable (Utilities|MakeSoftObjectPath (Utilities|String|Append (Variables|Default|GetAttributesRoot) (Variables|Default|GetAttributesRoot))) :!label _label))
            (bind _outxy (DataTable|EvaluateCurveTableRow _returnvalue_2 (Variables|/Game/Blueprints/Core/ActorBase.ActorBase_C|GetName (Variables|Default|GetOwner)) (Math|Conversions|ToFloat(Integer) (Variables|/Game/Blueprints/Core/ActorBase.ActorBase_C|GetLevel (Variables|Default|GetOwner))))
              (:RowFound
                (LocalVariables|SetL_CurrentValue _outxy))
              (:RowNotFound
                (return)))))
        (else
          (goto _label))))
    (:then_1
      (if (GameplayTags|HasTag (Variables|Default|GetTags) "(TagName=\"Attribute.Function.Max\")" true) ; 最大值限制
        (if (LocalVariables|GetL_HasSave)
          (bind (_value_2 _has_2) (Default|GetFloat (LocalVariables|GetL_Save) (Variables|/Game/Blueprints/Core/ActorBase.ActorBase_C|GetId (Variables|Default|GetOwner)) (Utilities|String|StringToName (Utilities|String|Append (GameplayTags|GetDebugStringfromGameplayTag (Variables|Default|GetTag)) "+" (GameplayTags|GetDebugStringfromGameplayTag "(TagName=\"Attribute.Function.Max\")")))))
          (if _has_2
            (LocalVariables|SetL_MaxValue _value_2)
            (else
              (bind _returnvalue_3 (Class|MyBlueprintFunctionLibrary|LoadCurveTable (Utilities|MakeSoftObjectPath (Utilities|String|Append (Variables|Default|GetAttributesRoot) (Variables|Default|GetAttributesRoot) "Max")) :!label _label_2))
              (bind _outxy_2 (DataTable|EvaluateCurveTableRow _returnvalue_3 (Variables|/Game/Blueprints/Core/ActorBase.ActorBase_C|GetName (Variables|Default|GetOwner)) (Math|Conversions|ToFloat(Integer) (Variables|/Game/Blueprints/Core/ActorBase.ActorBase_C|GetLevel (Variables|Default|GetOwner))))
                (:RowFound
                  (LocalVariables|SetL_MaxValue _outxy_2)))))
          (else
            (goto _label_2)))
        (Utilities|Map|Add (Variables|Default|GetFunctionValue) "(TagName=\"Attribute.Function.Max\")" (LocalVariables|GetL_MaxValue))))
    (:then_2
      (if (GameplayTags|HasTag (Variables|Default|GetTags) "(TagName=\"Attribute.Function.Min\")" true) ; 最小值限制
        (if (LocalVariables|GetL_HasSave)
          (bind (_value_3 _has_3) (Default|GetFloat (LocalVariables|GetL_Save) (Variables|/Game/Blueprints/Core/ActorBase.ActorBase_C|GetId (Variables|Default|GetOwner)) (Utilities|String|StringToName (Utilities|String|Append (GameplayTags|GetDebugStringfromGameplayTag (Variables|Default|GetTag)) "+" (GameplayTags|GetDebugStringfromGameplayTag "(TagName=\"Attribute.Function.Min\")")))))
          (if _has_3
            (LocalVariables|SetL_MinValue _value_3)
            (else
              (bind _returnvalue_4 (Class|MyBlueprintFunctionLibrary|LoadCurveTable (Utilities|MakeSoftObjectPath (Utilities|String|Append (Variables|Default|GetAttributesRoot) (Variables|Default|GetAttributesRoot) "Min")) :!label _label_3))
              (bind _outxy_3 (DataTable|EvaluateCurveTableRow _returnvalue_4 (Variables|/Game/Blueprints/Core/ActorBase.ActorBase_C|GetName (Variables|Default|GetOwner)) (Math|Conversions|ToFloat(Integer) (Variables|/Game/Blueprints/Core/ActorBase.ActorBase_C|GetLevel (Variables|Default|GetOwner))))
                (:RowFound
                  (LocalVariables|SetL_MinValue _outxy_3)))))
          (else
            (goto _label_3)))
        (Utilities|Map|Add (Variables|Default|GetFunctionValue) "(TagName=\"Attribute.Function.Min\")" (LocalVariables|GetL_MinValue))))
    (:then_3
      (bind _约束 (CallFunction|LimitValue (LocalVariables|GetL_CurrentValue)))
      (Variables|Default|SetCurrent (- _约束 1.0)) ; 故意设置不同值，以便触发变更事件
      (CallFunction|SetValue :NewValue _约束))))