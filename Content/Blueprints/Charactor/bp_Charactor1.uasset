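; Character Blueprint that gains a Move ability through its AbilityComponent on BeginPlay and animates its own relocation.
; The MoveShow event plays a timeline that shifts the actor toward a target location without sweeping.
; Each update blends from the current location rather than a stored start, so the track alpha compounds over the move.
; AttributeComponent setup nodes are present but unconnected, so they never run.
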(event Custom|MoveShow
  (params (NewLocation :type Vector))
  (bind _returnvalue (Transformation|GetActorLocation))
  (bind _新建轨道_0 (Timeline|时间轴_0 PlayFromStart)
    (:Update
      (Transformation|SetActorLocation (+ (* (- NewLocation _returnvalue) _新建轨道_0) _returnvalue) false false))))

(event EventBeginPlay
  (|CallParentFunction)
  (Default|Add能力 (Variables|Default|GetAbilityComponent) "(TagName=\"Ability.Move\")"))

(event Collision|EventActorBeginOverlap
  (params (OtherActor :type Actor%20Object%20Reference))
  (|CallParentFunction OtherActor) ; 此节点被禁用，将不会被调用。\n从引脚连出引线来编译功能。
)

(event EventTick
  (params (DeltaSeconds :type Float%20%28single-precision%29))
  (|CallParentFunction DeltaSeconds) ; 此节点被禁用，将不会被调用。\n从引脚连出引线来编译功能。
)

(fn ConstructionScript
  (|CallParentFunction))