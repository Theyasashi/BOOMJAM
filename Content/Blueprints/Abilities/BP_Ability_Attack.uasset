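; BP_Ability_Attack is an attack ability that plays a third-person attack animation on its owning character.
; On activation it requires a BP_TargetInfo_TargetObject target and a bp_Charactor1 owner, then plays ThirdPersonAttack_Montage on that character's skeletal mesh anim instance.
; CanActivate extends the parent check by also requiring Speed to be zero.
; The target serves only as a type gate; this graph applies no damage or other effect to it.
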(event EventOnActivate
  (params (Target :type BP%20Target%20Info%20Base%20Object%20Reference))
  (Utilities|Casting|CastToBP_TargetInfo_TargetObject Target)
  (bind _asbp_charactor_1 (Utilities|Casting|CastTobp_Charactor1 (Variables|Default|GetOwner)))
  (Animation|Montage|MontagePlay (Components|SkeletalMesh|GetAnimInstance (Variables|/Game/Blueprints/Charactor/bp_Charactor1.bp_Charactor1_C|GetSkeletalMesh _asbp_charactor_1)) "/Game/Mannequin/Animations/ThirdPersonAttack_Montage.ThirdPersonAttack_Montage" 1.0 "MontageLength" 0.0 true))

(fn CanActivate
  (params (Target :type BP%20Target%20Info%20Base%20Object%20Reference))
  (bind __ (|CallParentFunction Target))
  (return (and __ (== (Variables|Default|GetSpeed) 0.0))))