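; Grass hex tile actor for the HexSLG game that tracks the actor standing on it.
; The join event makes the incoming actor's previous tile Leave, then links tile and actor through ActorOnHexTile and StandHexTitle.
; Leave clears both references.
; Tick draws the tile's display name at its location as a debug string.
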(event Custom|join
  (params (ActorOnHexTile :type Actor%20Base%20Object%20Reference))
  (Utilities|IsValid (Variables|/Game/Blueprints/Core/ActorBase.ActorBase_C|GetStandHexTitle ActorOnHexTile)
    (:Is%20Valid
      (CallFunction|Leave (Variables|/Game/Blueprints/Core/ActorBase.ActorBase_C|GetStandHexTitle ActorOnHexTile)))
    (:Is%20Not%20Valid
      _))
  (Variables|Default|SetActorOnHexTile ActorOnHexTile)
  (Variables|/Game/Blueprints/Core/PlayerActorBase.PlayerActorBase_C|SetStandHexTitle ActorOnHexTile self))

(event Custom|Leave
  (Variables|/Game/Blueprints/Core/PlayerActorBase.PlayerActorBase_C|SetStandHexTitle (Variables|Default|GetActorOnHexTile) 0)
  (Variables|Default|SetActorOnHexTile 0))

(event EventBeginPlay)

(event Collision|EventActorBeginOverlap
  (params (OtherActor :type Actor%20Object%20Reference)))

(event EventTick
  (params (DeltaSeconds :type Float%20%28single-precision%29))
  (Rendering|Debug|DrawDebugString (Transformation|GetActorLocation) (Utilities|GetDisplayName self) 0 "(R=1.000000,G=1.000000,B=1.000000,A=1.000000)"))

(fn ConstructionScript)