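; BP_GridManager manages the tile grid and highlights the range a unit can move from an origin tile.
; On BeginPlay it broadcasts CreateFinish.
; ShowCanMoveHexTitle lazily gathers all Bp_HexTile_Grass actors, builds a diamond of array indices around the origin, then resets all move decals and enables those in range.
; Despite hex naming, it uses square-grid index math, assuming array order matches a hardcoded width-10 layout, without row-edge checks.
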(event EventBeginPlay
  (|CallParentFunction)
  (Default|CallCreateFinish))

(event Collision|EventActorBeginOverlap
  (params (OtherActor :type Actor%20Object%20Reference)))

(fn ConstructionScript)

(fn ShowCanMoveHexTitle
  (params (Range :type Integer) (OriginHexTitle :type Bp%20Hex%20Tile%20Grass%20Object%20Reference))
  (bind _canmovearr (LocalVariables|GetCanMoveArr))
  (if (Utilities|Array|IsValidIndex (Variables|Default|GetHexTiteArr))
    _
    (else
      (bind _outactors (Actor|GetAllActorsOfClass "/Game/SqrSLG/Blueprints/Bp_HexTile_Grass.Bp_HexTile_Grass_C"))
      (Variables|Default|SetHexTiteArr _outactors)))
  (for _index (range (- (Utilities|Array|FindItem (Variables|Default|GetHexTiteArr) OriginHexTitle) Range) (+ (Utilities|Array|FindItem (Variables|Default|GetHexTiteArr) OriginHexTitle) Range))
    (Utilities|Array|Add (LocalVariables|GetCanMoveArr) _index)
    (for _index_2 (range 1 (- Range (Math|Integer|Absolute(Integer) (- _index (Utilities|Array|FindItem (Variables|Default|GetHexTiteArr) OriginHexTitle)))))
      (Utilities|Array|Add _canmovearr (+ _index (* _index_2 (Class|KismetSystemLibrary|MakeLiteralInteger 10))))
      (Utilities|Array|Add _canmovearr (- _index (* _index_2 (Class|KismetSystemLibrary|MakeLiteralInteger 10))))))
  (for _array_element (Variables|Default|GetHexTiteArr)
    (Default|UpdateMoveDecal _array_element false))
  (for _array_element_2 (LocalVariables|GetCanMoveArr)
    (Utilities|IsValid (Utilities|Array|Get(acopy) (Variables|Default|GetHexTiteArr) _array_element_2)
      (:Is%20Valid
        (Default|UpdateMoveDecal (Utilities|Array|Get(acopy) (Variables|Default|GetHexTiteArr) _array_element_2) true)))))